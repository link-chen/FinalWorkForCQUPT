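; BP_Clock is a day-cycle controller that turns the level's directional light and keeps the sky in step with it.
; BeginPlay finds the directional lights, and each Signal event sets the first one's pitch from RotateNum, then calls ReturnNum.
; It then updates the Sky's sun direction and switches the light's intensity on or off depending on whether SunHeight is above or just below the horizon.
; Tick is unused.
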(event `self.ReceiveBeginPlay`
  (bind _outactors (`GameplayStatics.GetAllActorsOfClass` "/Script/Engine.DirectionalLight")))

(event `self.Signal`
  (bind _sky (`self.Sky`))
  (bind _output (`|GetArrayItem` (stale `self.ReceiveBeginPlay` _outactors)))
  (`self.K2_SetActorRotation` _output (`KismetMathLibrary.MakeRotator` 0.0 (- 300.0 (`self.RotateNum`))) false)
  (`self.ReturnNum`)
  (`/Engine/EngineSky/BP_Sky_Sphere.UpdateSunDirection` _sky)
  (if (>= (`/Engine/EngineSky/BP_Sky_Sphere.Sun height` _sky) -0.1)
    (bind _lightcomponent (`Light.LightComponent` _output))
    (`LightComponent.SetIntensity` _lightcomponent 1.0)
    (else
      (`LightComponent.SetIntensity` _lightcomponent 0.0))))

(fn `UserConstructionScript`)