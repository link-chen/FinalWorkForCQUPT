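; Cargo airplane actor that either flies into the map and opens its ramp, or takes off and closes it, depending on Enter.
; Chained timelines apply local offsets for movement and drive wheel and ramp alphas in the animation Blueprint, which Tick also updates for propellers.
; A box attaches overlapping cars to the plane's socket.
; A player leaving the box triggers a game mode event and closes the ramp.
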(event `self.ReceiveBeginPlay`
  ;[1 1 1] 获取动画蓝图
  (bind _asair_plan_animation_blue_print (cast `/Game/VigilanteContent/Vehicles/West_Transport_C130J/Anim/AirPlanAnimationBluePrint` (`SkeletalMeshComponent.GetAnimInstance` (`self.MeshComponent`))))
  (set `self.As Air Plan Animation Blue Print` _asair_plan_animation_blue_print))

(event `StartFly`
  (set `self.bFly` true :!label _label)
  (if (`self.bEnter`)
    (set `/Game/VigilanteContent/Vehicles/West_Transport_C130J/Anim/AirPlanAnimationBluePrint.WheelAlpha` 1.0 (`self.As Air Plan Animation Blue Print`))
    (`self.EnterMap`)
    (`KismetSystemLibrary.Delay` 18.0)
    (`self.OpenDoor`)
    (else
      (`self.Fly`))))

(event `self.CPPStartFly`
  (goto _label))

(event `EnterMap`
  ;[1 1 1] 入场轨迹
  (bind (_direction _x _z) (`Timeline|时间轴_4`)
    (:`Update`
      (`self.K2_AddActorLocalOffset` (`KismetMathLibrary.MakeVector` _x 0.0 _z)))
    (:`Finished`
      ;[1 1 1] 起飞轨迹
      (bind (_direction_2 _x_2 _z_2) (`Timeline|时间轴_0` :!label _label_2)
        (:`Update`
          (`self.K2_AddActorLocalOffset` (`KismetMathLibrary.MakeVector` _x_2 0.0 _z_2)))))))

(event `self.ReceiveTick`
  (params (DeltaSeconds :type "Float (single-precision)"))
  ;[1 1 1] 螺旋桨
  (if (`self.bFly`)
    (`/Game/VigilanteContent/Vehicles/West_Transport_C130J/Anim/AirPlanAnimationBluePrint.UpdateSpeed` (`self.As Air Plan Animation Blue Print`))))

(event `Fly`
  ;[1 1 1] 起飞轨迹
  (bind (_direction _x _z _wheel) (`Timeline|时间轴_1`)
    (:`Update`
      (set `/Game/VigilanteContent/Vehicles/West_Transport_C130J/Anim/AirPlanAnimationBluePrint.WheelAlpha` _wheel (`self.As Air Plan Animation Blue Print`))
      (`self.K2_AddActorLocalOffset` (`KismetMathLibrary.MakeVector` _x 0.0 _z)))
    (:`Finished`
      (`self.CloseDoor`)
      (goto _label_2))))

(event `CloseDoor`
  ;[1 1 1] 关机仓门
  (`KismetSystemLibrary.Delay` 5.0)
  (bind (_direction _x) (`Timeline|时间轴_2`)
    (:`Update`
      (set `/Game/VigilanteContent/Vehicles/West_Transport_C130J/Anim/AirPlanAnimationBluePrint.RampAlpha` _x (`self.As Air Plan Animation Blue Print`)))))

(event `self.Box.OnComponentBeginOverlap`
  (params (OverlappedComponent :type "PrimitiveComponent Object Reference") (OtherActor :type "Actor Object Reference") (OtherComp :type "PrimitiveComponent Object Reference") (OtherBodyIndex :type Integer) (bFromSweep :type Boolean) (SweepResult :type "HitResult Structure (by ref)"))
  ;[1 1 1] 挂载车辆
  (bind _asbp_base_car (cast `/Game/Source/Player/BP_Car/Car/BaseCar/BP_BaseCar` OtherActor))
  (`self.K2_AttachToActor` _asbp_base_car self "skeleton_grp插槽" "KeepWorld" "KeepWorld" "KeepWorld" true))

(event `OpenDoor`
  ;[1 1 1] 开机舱门
  (`KismetSystemLibrary.Delay` 5.0)
  (bind (_direction `_新建轨道_0`) (`Timeline|时间轴_3`)
    (:`Update`
      (set `/Game/VigilanteContent/Vehicles/West_Transport_C130J/Anim/AirPlanAnimationBluePrint.RampAlpha` `_新建轨道_0` (`self.As Air Plan Animation Blue Print`)))))

(event `self.Box.OnComponentEndOverlap`
  (params (OverlappedComponent :type "PrimitiveComponent Object Reference") (OtherActor :type "Actor Object Reference") (OtherComp :type "PrimitiveComponent Object Reference") (OtherBodyIndex :type Integer))
  ;[1 1 1] 判定玩家离开机舱
  (bind _asbp_player_charater_test (cast `/Game/Source/TPSSource/PlayerCharacter/BP_PlayerCharater_Test` OtherActor))
  (if (!= _asbp_player_charater_test (`self.As BP Player Charater Test`))
    (set `self.As BP Player Charater Test` _asbp_player_charater_test)
    (bind _asbp_tpsgame_mode_base (cast `/Game/Source/TPSSource/GameMode/BP_TPSGameModeBase` (`GameplayStatics.GetGameMode`)))
    (`/Game/Source/TPSSource/GameMode/BP_TPSGameModeBase.TriggerEvent` _asbp_tpsgame_mode_base)
    (`self.CloseDoor`)))

(fn `UserConstructionScript`)