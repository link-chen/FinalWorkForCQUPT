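; Test player character Blueprint that shows a TPS UI and can board BP_BaseCar vehicles.
; Capsule overlap with a car opens a Gate and end overlap closes it, so pressing E only works near a car.
; After a short delay, the controller possesses the car, which receives a player reference and calls ShowRunning, while the UI is removed.
; The AddUI function puts the widget back on the viewport.
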(event `self.ReceiveBeginPlay`
  (bind _returnvalue (`|CreateWidget` "/Game/Source/TPSSource/UI/TPSUI.TPSUI_C"))
  (bind _output_get (set `self.UI` _returnvalue))
  (`UserWidget.AddToViewport` _output_get 0))

(event `self.Capsule.OnComponentBeginOverlap`
  (params (OverlappedComponent :type "PrimitiveComponent Object Reference") (OtherActor :type "Actor Object Reference") (OtherComp :type "PrimitiveComponent Object Reference") (OtherBodyIndex :type Integer) (bFromSweep :type Boolean) (SweepResult :type "HitResult Structure (by ref)"))
  (bind _asbp_base_car (cast `/Game/Source/Player/BP_Car/Car/BaseCar/BP_BaseCar` OtherActor))
  (goto _label :!via `Open`))

(event `Key|E`
  (params (Key :type "Key Structure"))
  (:`Pressed`
    (`/Engine/EditorBlueprintResources/StandardMacros.Gate` true :!label _label
      (:`Exit`
        (`KismetSystemLibrary.Delay` 0.2)
        (`Controller.Possess` (`GameplayStatics.GetPlayerController` 0) (stale `self.Capsule.OnComponentBeginOverlap` _asbp_base_car))
        (set `/Game/Source/Player/BP_Car/Car/BaseCar/BP_BaseCar.Player` self (stale `self.Capsule.OnComponentBeginOverlap` _asbp_base_car))
        (`BaseCar.ShowRunning` (stale `self.Capsule.OnComponentBeginOverlap` _asbp_base_car))
        (`Widget.RemoveFromParent` (`self.UI`))))))

(event `self.Capsule.OnComponentEndOverlap`
  (params (OverlappedComponent :type "PrimitiveComponent Object Reference") (OtherActor :type "Actor Object Reference") (OtherComp :type "PrimitiveComponent Object Reference") (OtherBodyIndex :type Integer))
  (cast `/Game/Source/Player/BP_Car/Car/BaseCar/BP_BaseCar` OtherActor)
  (goto _label :!via `Close`))

(fn `AddUI`
  (`UserWidget.AddToViewport` (`self.UI`) 0))

(fn `UserConstructionScript`)